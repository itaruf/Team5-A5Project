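; BP_RollingDonut is a physics donut placeable that launches itself once when hit by a tagged actor.
; On a component hit, it checks the other actor for the configured tag and uses an IsActive flag to ignore later hits.
; The first valid hit replaces the donut's linear velocity with the Impulse value, while BeginPlay only calls the parent.
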(event `self.ReceiveBeginPlay`
  (`parent.ReceiveBeginPlay`))

(event `self.Donut.OnComponentHit`
  (params (HitComponent :type "PrimitiveComponent Object Reference") (OtherActor :type "Actor Object Reference") (OtherComp :type "PrimitiveComponent Object Reference") (NormalImpulse :type "Vector Structure") (Hit :type "HitResult Structure (by ref)"))
  (if (`self.ActorHasTag` OtherActor (`self.Tag`))
    (if (not (`self.Is Active`))
      (set `self.Is Active` true)
      (bind _output_get (set `self.Impulse` (`self.Impulse`)))
      (`PrimitiveComponent.SetPhysicsLinearVelocity` (`self.Donut`) _output_get false "None"))))

(fn `UserConstructionScript`)