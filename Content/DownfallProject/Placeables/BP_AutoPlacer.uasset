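; Placeable actor that snaps itself to the surface below on BeginPlay, plus an offset, unless deactivated.
; A second trace on another channel rejects the spot if it hits higher than that surface.
; Rejected spots or missed ground trigger TryRespawn, which traces down from random points in the Box bounds to relocate, destroying the actor once MaxTry is reached.
; Overlapping a BP_DestroyProps actor also destroys it.
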(event `self.ReceiveBeginPlay`
  (bind (_returnvalue_x _returnvalue_y _returnvalue_z) (`KismetMathLibrary.BreakVector` (`self.K2_GetActorLocation` self)))
  (if (not (`self.IsDeactivated`))
    (bind _outhit (`KismetSystemLibrary.LineTraceSingle` (`KismetMathLibrary.MakeVector` _returnvalue_x _returnvalue_y _returnvalue_z) (`KismetMathLibrary.MakeVector` _returnvalue_x _returnvalue_y (- _returnvalue_z 10000.0)) "TraceTypeQuery3" :!label _label))
    (bind _outhit_2 (`KismetSystemLibrary.LineTraceSingle` (`KismetMathLibrary.MakeVector` _returnvalue_x _returnvalue_y (+ _returnvalue_z 500.0)) (`KismetMathLibrary.MakeVector` 0.0 0.0 (- _returnvalue_z 10000.0)) "TraceTypeQuery5"))
    (if (and (`GameplayStatics.BreakHitResult` _outhit_2) (< (.z (`.ImpactPoint` (`GameplayStatics.BreakHitResult` _outhit))) (.z (`.ImpactPoint` (`GameplayStatics.BreakHitResult` _outhit_2)))))
      (if (!= (`self.ComptMaxTry`) (`self.MaxTry`)) :!label _label_2
        (`self.TryRespawn`)
        (goto _label)
        (else
          (`self.K2_DestroyActor`)))
      (elif (`GameplayStatics.BreakHitResult` _outhit)
        (`self.K2_SetActorLocation` (`KismetMathLibrary.MakeVector` (.x (`.ImpactPoint` (`GameplayStatics.BreakHitResult` _outhit))) (.y (`.ImpactPoint` (`GameplayStatics.BreakHitResult` _outhit))) (+ (.z (`.ImpactPoint` (`GameplayStatics.BreakHitResult` _outhit))) (`self.Offset`))) false true)
        (else
          (goto _label_2))))))

(event `self.ReceiveActorBeginOverlap`
  (params (OtherActor :type "Actor Object Reference"))
  (cast `/Game/DownfallProject/Core/CharacterBehaviour/BP_DestroyProps` OtherActor)
  (`self.K2_DestroyActor`))

(fn `TryRespawn`
  (bind (_origin _boxextent) (`KismetSystemLibrary.GetComponentBounds` (`self.Box`)))
  (bind (_returnvalue_x _returnvalue_y _returnvalue_z) (`KismetMathLibrary.BreakVector` (`KismetMathLibrary.RandomPointInBoundingBox` _origin _boxextent)))
  (bind _returnvalue (+ _returnvalue_z 100000.0))
  (`/Engine/EditorBlueprintResources/StandardMacros.IncrementInt` (`self.ComptMaxTry`)
    (:`  `
      (bind (_outhit _returnvalue_2) (`KismetSystemLibrary.LineTraceSingleForObjects` (`KismetMathLibrary.MakeVector` _returnvalue_x _returnvalue_y _returnvalue) (+ (`KismetMathLibrary.MakeVector` _returnvalue_x _returnvalue_y _returnvalue) (* (* (`self.GetActorUpVector`) -1) 150000)) (`self.AttachToObj`)))
      (if _returnvalue_2
        (`self.K2_SetActorLocation` (`.ImpactPoint` (`GameplayStatics.BreakHitResult` _outhit)) false true)))))

(fn `UserConstructionScript`)