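; BP_QTE_Jump is a trigger actor that shows and hides a jump quick-time-event prompt for the ALS AnimMan character.
; When that character enters the Trigger volume, the Widget component's Widget_QTE_Jump runs DisplayHUD, and leaving the volume runs FadeHUD.
; The actor only drives the prompt's visibility and contains no input or jump logic itself.
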(event `self.Trigger.OnComponentBeginOverlap`
  (params (OverlappedComponent :type "PrimitiveComponent Object Reference") (OtherActor :type "Actor Object Reference") (OtherComp :type "PrimitiveComponent Object Reference") (OtherBodyIndex :type Integer) (bFromSweep :type Boolean) (SweepResult :type "HitResult Structure (by ref)"))
  (bind _asals_anim_man_character_bp (cast `/Game/AdvancedLocomotionV4/Blueprints/CharacterLogic/ALS_AnimMan_CharacterBP` OtherActor))
  (if (== OtherActor _asals_anim_man_character_bp)
    (bind _aswidget_qte_jump (cast `/Game/DownfallProject/QTE/Widget_QTE_Jump` (`WidgetComponent.GetWidget` (`self.Widget`))))
    (`/Game/DownfallProject/QTE/Widget_QTE_Jump.DisplayHUD` _aswidget_qte_jump)))

(event `self.Trigger.OnComponentEndOverlap`
  (params (OverlappedComponent :type "PrimitiveComponent Object Reference") (OtherActor :type "Actor Object Reference") (OtherComp :type "PrimitiveComponent Object Reference") (OtherBodyIndex :type Integer))
  (bind _asals_anim_man_character_bp (cast `/Game/AdvancedLocomotionV4/Blueprints/CharacterLogic/ALS_AnimMan_CharacterBP` OtherActor))
  (if (== OtherActor _asals_anim_man_character_bp)
    (bind _aswidget_qte_jump (cast `/Game/DownfallProject/QTE/Widget_QTE_Jump` (`WidgetComponent.GetWidget` (`self.Widget`))))
    (`/Game/DownfallProject/QTE/Widget_QTE_Jump.FadeHUD` _aswidget_qte_jump)))

(fn `UserConstructionScript`)