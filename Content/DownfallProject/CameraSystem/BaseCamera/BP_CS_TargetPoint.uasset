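; Camera-system target point that records its own rotation and a yaw offset relative to the player pawn when play begins.
; The offset is the angle in degrees between both forward vectors, negated when their dot product is negative, so the sign marks facing away rather than left or right.
; Tick is empty, and the timeline rotation blend and control-rotation logic are disconnected and never run.
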(event `self.ReceiveBeginPlay`
  (set `self.Rotation` (`self.K2_GetActorRotation`))
  (bind _returnvalue (`self.CalculateYawOffset`))
  (set `self.YawOffset` _returnvalue))

(event `self.ReceiveTick`
  (params (DeltaSeconds :type "Float (single-precision)")))

(fn `CalculateYawOffset`
  (returns (ReturnValue :type "Float (double-precision)"))
  (bind _returnvalue (`KismetMathLibrary.Dot_VectorVector` (`KismetMathLibrary.GetForwardVector` (`self.K2_GetActorRotation`)) (`self.GetActorForwardVector` (`GameplayStatics.GetPlayerPawn` 0))))
  (bind _returnvalue_2 (`KismetMathLibrary.DegAcos` _returnvalue))
  (if (< _returnvalue 0.0)
    (return (* _returnvalue_2 -1.0))
    (else
      (return _returnvalue_2))))

(fn `UserConstructionScript`)