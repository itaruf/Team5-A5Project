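; AC_Camera is a base camera component that holds references to the player and its camera-related objects.
; A custom event calls SetData, then stores the game mode cast to ALS_GameMode_SP.
; SetData copies the Player, PlayerController and PlayerCameraManager from that stored game mode reference, so it reads GameMode before this event assigns it.
; It contains no camera movement or view logic.
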(event `CustomEvent`
  (`self.Set Data`)
  (set `self.Game Mode` (cast `/Game/AdvancedLocomotionV4/Blueprints/GameModes/ALS_GameMode_SP` (`GameplayStatics.GetGameMode`) :!pure true)))

(event `Set Data`
  (`|ExecutionSequence`
    (:`then_0`
      (set `self.Player` (`/Game/AdvancedLocomotionV4/Blueprints/GameModes/ALS_GameMode_SP.Player` (`self.Game Mode`)))
      (set `self.Player Controller` (`/Game/AdvancedLocomotionV4/Blueprints/GameModes/ALS_GameMode_SP.PlayerController` (`self.Game Mode`)))
      (set `self.Player Camera Manager` (`/Game/AdvancedLocomotionV4/Blueprints/GameModes/ALS_GameMode_SP.PlayerCameraManager` (`self.Game Mode`))))))