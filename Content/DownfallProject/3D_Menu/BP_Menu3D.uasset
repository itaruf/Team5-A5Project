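; BP_Menu3D is one screen of a 3D menu, a world-placed actor that shows a widget and serves as a camera view target.
; On BeginPlay it disables its collision and binds to the menu widget's link-transition event.
; That event passes an index into LinkedMenus to pick the next menu actor.
; Transitions move collision from the current menu to the target and smoothly blend the player's view to it.
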(event `self.ReceiveBeginPlay`
  (bind _aswidjet_menu_3d (cast `/Game/DownfallProject/3D_Menu/Widjet/Widjet_Menu3D` (`WidgetComponent.GetUserWidgetObject` (`self.Widget`))))
  (add `/Game/DownfallProject/3D_Menu/Widjet/Widjet_Menu3D.TransitionToLinkMenu` _aswidjet_menu_3d (delegate `OnTransitionBetweenMenus`))
  (`self.SetActorEnableCollision` false))

(event `OnTransitionBetweenMenus`
  (params (MenuIndex :type Integer))
  (if (`KismetArrayLibrary.Array_IsValidIndex` (`self.LinkedMenus`) MenuIndex)
    (`self.TransitionTo` (`|GetArrayItem` (`self.LinkedMenus`) MenuIndex))))

(event `TransitionTo`
  (params (BPMenu3D :type "/Game/DownfallProject/3D_Menu/BP_Menu3D Object Reference"))
  (`self.SetActorEnableCollision` false)
  (`self.SetActorEnableCollision` BPMenu3D true)
  (`PlayerController.SetViewTargetWithBlend` (`GameplayStatics.GetPlayerController` 0) BPMenu3D 2.0 "VTBlend_EaseInOut" 2.0 false))

(fn `UserConstructionScript`)