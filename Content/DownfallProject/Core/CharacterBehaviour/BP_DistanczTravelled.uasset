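; Actor Blueprint that tracks the total distance it has travelled since BeginPlay.
; BeginPlay stores the starting location and starts AddDistance, a custom event that re-calls itself after a short Delay instead of using Tick.
; Each pass adds the length of the movement since the last sample to Distance, then stores the current location for the next one.
; Nothing in this graph reads or displays the accumulated total.
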(event `self.ReceiveBeginPlay`
  (set `self.Location` (`self.K2_GetActorLocation`))
  (`self.Add Distance`))

(event `Add Distance`
  (set `self.Distance` (+ (`KismetMathLibrary.VSize` (- (`self.Location`) (`self.K2_GetActorLocation`))) (`self.Distance`)))
  (set `self.Location` (`self.K2_GetActorLocation`))
  (`KismetSystemLibrary.Delay` 0.01)
  (`self.Add Distance`))

(fn `UserConstructionScript`)