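; Box-volume scatter actor that randomly places objects onto surfaces below it.
; The construction script sizes the box from Scale, defaulting it when zero.
; Spawn runs Counter downward traces from high above random box points, filtered by AttachToObj, and randomly adds a Mesh2 instance or spawns a Mesh1 actor at each hit with random yaw.
; BeginPlay is empty, and a duplicate of the Spawn logic sits disconnected in the event graph.
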(event `self.ReceiveBeginPlay`)

(fn `Spawn`
  (bind _returnvalue (`KismetMathLibrary.RandomFloatInRange` 0.0 (`self.MaxRotation`)))
  (bind (_origin _boxextent) (`KismetSystemLibrary.GetComponentBounds` (`self.Box`)))
  (bind (_returnvalue_x _returnvalue_y _returnvalue_z) (`KismetMathLibrary.BreakVector` (`KismetMathLibrary.RandomPointInBoundingBox` _origin _boxextent)))
  (bind _returnvalue_2 (+ _returnvalue_z 100000.0))
  (`|ExecutionSequence`
    (:`then_0`
      (`StaticMeshComponent.SetStaticMesh` (`self.InstancedStaticMesh`) (`self.Mesh2`)))
    (:`then_1`
      (for _ (range (`self.Counter`))
        (bind (_outhit _returnvalue_3) (`KismetSystemLibrary.LineTraceSingleForObjects` (`KismetMathLibrary.MakeVector` _returnvalue_x _returnvalue_y _returnvalue_2) (+ (`KismetMathLibrary.MakeVector` _returnvalue_x _returnvalue_y _returnvalue_2) (* (* (`self.GetActorUpVector`) -1) 150000)) (`self.AttachToObj`)))
        (if _returnvalue_3
          (if (== (`KismetMathLibrary.RandomIntegerInRange` 0 1) 0)
            (bind (_bblockinghit _binitialoverlap _time _distance _location _impactpoint) (`GameplayStatics.BreakHitResult` _outhit))
            (`InstancedStaticMeshComponent.AddInstance` (`self.InstancedStaticMesh`) (`KismetMathLibrary.MakeTransform` _impactpoint (`KismetMathLibrary.MakeRotator` 0.0 0.0 _returnvalue)) true)
            (else
              (`|SpawnActorFromClass` (`self.Mesh1`) (`KismetMathLibrary.MakeTransform` _impactpoint (`KismetMathLibrary.MakeRotator` 0.0 0.0 _returnvalue)) "Undefined" "OverrideRootScale" null null))))))))

(fn `UserConstructionScript`
  (if (== (`self.Scale`) (0.0 0.0 0.0))
    (set `self.Scale` (500.0 500.0 500.0)))
  (`BoxComponent.SetBoxExtent` (`self.Box`) (`self.Scale`) true))