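; Procedural terrain tile that chains copies of itself along Y to extend the map as the player advances.
; The first tile builds a random-height vertex grid into a collidable ProceduralMesh with a random material, re-rolled on Tick while invalid.
; Once the player is far enough along +Y, it spawns and fills the next tile once.
; Saved edge heights seed the new tile's first row so the seams line up.
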(event `self.ReceiveBeginPlay`
  (bind _material (`self.Material`))
  (bind _material_2 (`self.Material`))
  (if (`self.FirstSpace`)
    (`self.EnableInput` (`GameplayStatics.GetPlayerController` 0))
    (`PrimitiveComponent.SetMaterial` (`self.ProceduralMesh`) 0 (`|GetArrayItem` _material (`KismetMathLibrary.RandomIntegerInRange` 0 (`KismetArrayLibrary.Array_Length` _material))))
    (`self.CreateMap`)
    (`self.CreateTriangles`)
    (`ProceduralMeshComponent.CreateMeshSection_LinearColor` :`self` (`self.ProceduralMesh`) :`Vertices` (`self.Vertices`) :`Triangles` (`self.Triangles`) :`UV0` (`self.UV0`) :`bCreateCollision` true)
    (`PrimitiveComponent.SetMaterial` (`self.ProceduralMesh`) 0 (`|GetArrayItem` _material_2 (`KismetMathLibrary.RandomIntegerInRange` 0 (`KismetArrayLibrary.Array_Length` _material_2))))))

(event `self.ReceiveTick`
  (params (DeltaSeconds :type "Float (single-precision)"))
  (bind (_returnvalue_x _returnvalue_y) (`KismetMathLibrary.BreakVector` (`self.K2_GetActorLocation`)))
  (bind _material (`self.Material`))
  (bind (_returnvalue_x_2 _returnvalue_y_2) (`KismetMathLibrary.BreakVector` (`SceneComponent.K2_GetComponentLocation` (`Character.CapsuleComponent` (`GameplayStatics.GetPlayerCharacter` 0)))))
  (`|ExecutionSequence`
    (:`then_0`
      (if (`self.Dead`)
        _
        (elif (> _returnvalue_y_2 _returnvalue_y)
          (if (>= (`self.GetDistanceTo` (`GameplayStatics.GetPlayerCharacter` 0) self) (* (/ (`self.YSize`) 2) (`self.ScaleX`)))
            (set `self.Dead` true)
            (`self.CreateNewSpace`)))))
    (:`then_1`
      (if (not (`KismetSystemLibrary.IsValid` (`PrimitiveComponent.GetMaterial` (`self.ProceduralMesh`) 0)))
        (`PrimitiveComponent.SetMaterial` (`self.ProceduralMesh`) 0 (`|GetArrayItem` _material (`KismetMathLibrary.RandomIntegerInRange` 0 (`KismetArrayLibrary.Array_Length` _material))))))))

(fn `CreateMap`
  (locals (X :type Integer) (Y :type Integer))
  (bind _vertices (`self.Vertices`))
  (for _index (range (+ (`self.XSize`) 1))
    (set `local.X` _index)
    (for _index_2 (range (+ (`self.YSize`) 1))
      (set `local.Y` _index_2)
      (`KismetArrayLibrary.Array_Add` (`self.Vertices`) (`KismetMathLibrary.MakeVector` (* (`local.X`) (`self.ScaleX`)) (* (`local.Y`) (`self.ScaleY`)) (`KismetMathLibrary.RandomFloatInRange` (`self.ZMin`) (`self.ZMax`))))
      (`KismetArrayLibrary.Array_Add` (`self.UV0`) (`KismetMathLibrary.MakeVector2D` (* (`local.X`) (`self.UVScale`)) (* (`local.Y`) (`self.UVScale`))))
      (`KismetSystemLibrary.DrawDebugBox` (`KismetMathLibrary.MakeVector` (* (`local.X`) (`self.ScaleX`)) (* (`local.Y`) (`self.ScaleY`))) (0.0 0.0 0.0) (struct :`A` 1.0)))
    (`KismetArrayLibrary.Array_Add` (`self.VerticeForNextSpace`) (`|GetArrayItem` _vertices (- (`KismetArrayLibrary.Array_Length` _vertices) 1)))))

(fn `CreateNewSpace`
  (locals (X :type Integer) (Y :type Integer) (Compt :type Integer))
  (bind _verticefornextspace (`self.VerticeForNextSpace`))
  (bind _compt (`local.Compt`))
  (bind (_returnvalue_x _returnvalue_y) (`KismetMathLibrary.BreakVector` (`SceneComponent.K2_GetComponentLocation` (`self.ProceduralMesh`))))
  (bind (_output_x _output_y _output_z) (`KismetMathLibrary.BreakVector` (`|GetArrayItem` _verticefornextspace)))
  (bind _returnvalue (`|SpawnActorFromClass` "BP_MapSpawner_C" (`KismetMathLibrary.MakeTransform` (`KismetMathLibrary.MakeVector` 0.0 (+ _returnvalue_y (* (`self.YSize`) (`self.ScaleY`))))) "Undefined" "OverrideRootScale" null null))
  (bind _material (`/Game/DownfallProject/Core/BP_MapSpawner.Material` _returnvalue))
  (`PrimitiveComponent.SetMaterial` (`/Game/DownfallProject/Core/BP_MapSpawner.ProceduralMesh` _returnvalue) 0 (`|GetArrayItem` _material (`KismetMathLibrary.RandomIntegerInRange` 0 (`KismetArrayLibrary.Array_Length` _material))))
  (for _index (range (+ (`self.XSize`) 1))
    (set `local.X` _index)
    (for _index_2 (range (+ (`self.YSize`) 1))
      (set `local.Y` _index_2)
      (if (or (== _compt 0) (== (mod _compt (+ (`self.YSize`) 1)) 0))
        (`KismetArrayLibrary.Array_Add` (`/Game/DownfallProject/Core/BP_MapSpawner.Vertices` _returnvalue) (`KismetMathLibrary.MakeVector` (* (`local.X`) (`self.ScaleX`)) (* (`local.Y`) (`self.ScaleY`)) _output_z))
        (`KismetArrayLibrary.Array_Remove` _verticefornextspace)
        (`/Engine/EditorBlueprintResources/StandardMacros.IncrementInt` (`local.Compt`))
        (else
          (`KismetArrayLibrary.Array_Add` (`/Game/DownfallProject/Core/BP_MapSpawner.Vertices` _returnvalue) (`KismetMathLibrary.MakeVector` (* (`local.X`) (`self.ScaleX`)) (* (`local.Y`) (`self.ScaleY`)) (`KismetMathLibrary.RandomFloatInRange` (`self.ZMin`) (`self.ZMax`))))
          (`KismetArrayLibrary.Array_Add` (`/Game/DownfallProject/Core/BP_MapSpawner.UV0` _returnvalue) (`KismetMathLibrary.MakeVector2D` (* (`local.X`) (`self.UVScale`)) (* (`local.Y`) (`self.UVScale`))))
          (`KismetSystemLibrary.DrawDebugBox` (`KismetMathLibrary.MakeVector` (* (`local.X`) (`self.ScaleX`)) (* (`local.Y`) (`self.ScaleY`))) (0.0 0.0 0.0) (struct :`A` 1.0))
          (`/Engine/EditorBlueprintResources/StandardMacros.IncrementInt` (`local.Compt`)))))
    (bind _vertices (`/Game/DownfallProject/Core/BP_MapSpawner.Vertices` _returnvalue))
    (`KismetArrayLibrary.Array_Add` (`/Game/DownfallProject/Core/BP_MapSpawner.VerticeForNextSpace` _returnvalue) (`|GetArrayItem` _vertices (- (`KismetArrayLibrary.Array_Length` _vertices) 1))))
  (`self.CreateTriangles` _returnvalue)
  (`ProceduralMeshComponent.CreateMeshSection_LinearColor` :`self` (`/Game/DownfallProject/Core/BP_MapSpawner.ProceduralMesh` _returnvalue) :`Vertices` (`/Game/DownfallProject/Core/BP_MapSpawner.Vertices` _returnvalue) :`Triangles` (`/Game/DownfallProject/Core/BP_MapSpawner.Triangles` _returnvalue) :`UV0` (`/Game/DownfallProject/Core/BP_MapSpawner.UV0` _returnvalue) :`bCreateCollision` true))

(fn `CreateTriangles`
  (locals (Vertex :type Integer))
  (for _ (range (`self.XSize`))
    (for _ (range (`self.YSize`))
      (`KismetArrayLibrary.Array_Add` (`self.Triangles`) (`local.Vertex`))
      (`KismetArrayLibrary.Array_Add` (`self.Triangles`) (+ (`local.Vertex`) 1))
      (`KismetArrayLibrary.Array_Add` (`self.Triangles`) (+ (`self.YSize`) 1 (`local.Vertex`)))
      (`KismetArrayLibrary.Array_Add` (`self.Triangles`) (+ (`local.Vertex`) 1))
      (`KismetArrayLibrary.Array_Add` (`self.Triangles`) (+ (`self.YSize`) 2 (`local.Vertex`)))
      (`KismetArrayLibrary.Array_Add` (`self.Triangles`) (+ (`self.YSize`) 1 (`local.Vertex`)))
      (`/Engine/EditorBlueprintResources/StandardMacros.IncrementInt` (`local.Vertex`)))
    (`/Engine/EditorBlueprintResources/StandardMacros.IncrementInt` (`local.Vertex`))))

(fn `UserConstructionScript`)