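; BP_MapSpawner generates an endless chain of procedural terrain tiles along Y as the player advances.
; Each tile uses a rarity-weighted setting to build a random-height ProceduralMesh, optionally carves a wandering river, and spawns BP_SpawnObjectOnMap to populate it.
; When the player nears, it spawns the next tile, passing edge vertices for seamless joins and periodically multiplying spawn counts for difficulty.
; Spent tiles destroy themselves once the player is far away.
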(event `self.ReceiveBeginPlay`
  (bind (_returnvalue_x _returnvalue_y _returnvalue_z) (`KismetMathLibrary.BreakVector` (`self.K2_GetActorLocation`)))
  (bind (_settings_enum _settings_landsettings _settings_spawnersettings) (break `/Game/DownfallProject/Core/Map/Settings/ST_MapSettings` (`self.Settings`)))
  (bind _settings (`/Game/DownfallProject/Core/Map/Settings/MapSettings.Settings` (`self.MapSettingsActor`)))
  (bind _settings_2 (`/Game/DownfallProject/Core/Map/Settings/MapSettings.Settings` (`self.MapSettingsActor`)))
  (bind _returnvalue (`KismetArrayLibrary.Array_Length` _settings_2))
  (set `self.Player` (`GameplayStatics.GetPlayerCharacter` 0))
  (if (`self.FirstSpace`)
    (for _index (range (+ _returnvalue 1))
      (bind (_output_enum _output_landsettings _output_spawnersettings _output_rarity) (break `/Game/DownfallProject/Core/Map/Settings/ST_MapSettings` (`|GetArrayItem` _settings_2 _index)))
      (set `self.TempRarity` (+ _output_rarity (`self.TempRarity`))))
    (bind _output_get (set `self.TempRarity` (`KismetMathLibrary.RandomIntegerInRange` 0 (`self.TempRarity`))))
    (for _index_2 (range (+ _returnvalue 1))
      (bind (_output_enum_2 _output_landsettings_2 _output_spawnersettings_2 _output_rarity_2) (break `/Game/DownfallProject/Core/Map/Settings/ST_MapSettings` (`|GetArrayItem` (`/Game/DownfallProject/Core/Map/Settings/MapSettings.Settings` (`self.MapSettingsActor`)) _index_2)))
      (if (<= _output_get _output_rarity_2)
        (break)
        (else
          (set `self.TempRarity` (- (`self.TempRarity`) _output_rarity_2)))))
    (bind _output (`|GetArrayItem` _settings _index_2))
    (set `self.YSize` (`.YSize_16_236BBE6B408435D9FF59C4AC3005C7D5` (break `/Game/DownfallProject/Core/Map/Settings/ST_LandSettings` (`.LandSettings_10_C2292C68434BF2A2A2BC62AEF734BE6D` (break `/Game/DownfallProject/Core/Map/Settings/ST_MapSettings` _output)))))
    (set `self.UVScale` (`.UVScale_19_40BA05704A7CF0A676E13FB8252BB641` (break `/Game/DownfallProject/Core/Map/Settings/ST_LandSettings` (`.LandSettings_10_C2292C68434BF2A2A2BC62AEF734BE6D` (break `/Game/DownfallProject/Core/Map/Settings/ST_MapSettings` _output)))))
    (set `self.ZMin` (`.ZMin_20_EBE479EB4E5073A8409F7B9CB26DAF67` (break `/Game/DownfallProject/Core/Map/Settings/ST_LandSettings` (`.LandSettings_10_C2292C68434BF2A2A2BC62AEF734BE6D` (break `/Game/DownfallProject/Core/Map/Settings/ST_MapSettings` _output)))))
    (set `self.ZMax` (`.ZMax_21_6862E78A47B566DFAEF57B9A59C42546` (break `/Game/DownfallProject/Core/Map/Settings/ST_LandSettings` (`.LandSettings_10_C2292C68434BF2A2A2BC62AEF734BE6D` (break `/Game/DownfallProject/Core/Map/Settings/ST_MapSettings` _output)))))
    (set `self.Settings` (`|GetArrayItem` _settings _index_2))
    (`self.Create Map`)
    (`self.CreateTriangles`)
    (`ProceduralMeshComponent.CreateMeshSection_LinearColor` :`self` (`self.ProceduralMesh`) :`Vertices` (`self.Vertices`) :`Triangles` (`self.Triangles`) :`UV0` (`self.UV0`) :`bCreateCollision` true)
    (bind _returnvalue_2 (`|SpawnActorFromClass` "/Game/DownfallProject/Core/Map/BP_SpawnObjectOnMap.BP_SpawnObjectOnMap_C" (`KismetMathLibrary.MakeTransform` (`KismetMathLibrary.MakeVector` (+ (/ (* (`self.XSize`) (`self.ScaleX`)) 2.0) _returnvalue_x) (+ _returnvalue_y (/ (* (`self.YSize`) (`self.ScaleY`)) 2.0)) (+ _returnvalue_z (`self.ZMax`))) (struct) (`KismetMathLibrary.MakeVector` (/ (* (`self.XSize`) (`self.ScaleX`)) 1000.0) (/ (* (`self.YSize`) (`self.ScaleY`)) 1000.0) 1.0)) "Undefined" "OverrideRootScale" null null))
    (`self.K2_AttachToActor` _returnvalue_2 self "None" "KeepRelative" "KeepRelative" "KeepRelative" true)
    (set `/Game/DownfallProject/Core/Map/BP_SpawnObjectOnMap.Settings` _settings_spawnersettings _returnvalue_2)
    (`/Game/DownfallProject/Core/Map/BP_SpawnObjectOnMap.Spawn` _returnvalue_2)
    (`PrimitiveComponent.SetMaterial` (`self.ProceduralMesh`) 0 (break `/Game/DownfallProject/Core/Map/Settings/ST_LandSettings` (`.LandSettings_10_C2292C68434BF2A2A2BC62AEF734BE6D` (break `/Game/DownfallProject/Core/Map/Settings/ST_MapSettings` (`self.Settings`)))))
    (set `self.ObjectSpawner` _returnvalue_2)
    (`/Engine/EditorBlueprintResources/StandardMacros.IncrementInt` (`self.NbMap`)
      (:`  `
        (set `self.EndConstruct` true)))))

(event `self.ReceiveTick`
  (params (DeltaSeconds :type "Float (single-precision)"))
  (bind _ysize (`self.YSize`))
  (if (`KismetSystemLibrary.IsValid` (`self.Player`))
    (if (`self.Dead`)
      (if (>= (`self.GetDistanceTo` (`self.Player`) self) (* (+ _ysize (/ _ysize 2)) (`self.ScaleY`)))
        (`self.K2_DestroyActor` (`self.ObjectSpawner`))
        (`self.K2_DestroyActor` self))
      (elif (`self.EndConstruct`)
        (if (and (>= (`self.GetDistanceTo` (`self.Player`) self) 0.0) (< (`self.GetDistanceTo` (`self.Player`) self) (* (`self.YSize`) (`self.ScaleY`))))
          (set `self.Dead` true)
          (`self.CreateNewSpace`))))
    (else
      (set `self.Player` (`GameplayStatics.GetPlayerCharacter` 0)))))

(fn `Create Map`
  (locals (X :type Integer) (Y :type Integer))
  (bind _returnvalue (`KismetMathLibrary.RandomIntegerInRange` 0 2))
  (bind _vertices (`self.Vertices`))
  (bind _settings (`self.Settings`))
  (bind _settings_2 (`self.Settings`))
  (bind _verticefornextspace (`self.VerticeForNextSpace`))
  (bind _returnvalue_2 (+ (`self.XRiver`) 1))
  (for _index (range (+ (`self.XSize`) 1))
    (set `local.X` _index)
    (for _index_2 (range (+ (`.YSize_16_236BBE6B408435D9FF59C4AC3005C7D5` (break `/Game/DownfallProject/Core/Map/Settings/ST_LandSettings` (`.LandSettings_10_C2292C68434BF2A2A2BC62AEF734BE6D` (break `/Game/DownfallProject/Core/Map/Settings/ST_MapSettings` _settings_2)))) 1))
      (set `local.Y` _index_2)
      (`KismetArrayLibrary.Array_Add` (`self.Vertices`) (`KismetMathLibrary.MakeVector` (* (`local.X`) (`self.ScaleX`)) (* (`local.Y`) (`self.ScaleY`)) (`KismetMathLibrary.RandomFloatInRange` (`.ZMin_20_EBE479EB4E5073A8409F7B9CB26DAF67` (break `/Game/DownfallProject/Core/Map/Settings/ST_LandSettings` (`.LandSettings_10_C2292C68434BF2A2A2BC62AEF734BE6D` (break `/Game/DownfallProject/Core/Map/Settings/ST_MapSettings` _settings_2)))) (`.ZMax_21_6862E78A47B566DFAEF57B9A59C42546` (break `/Game/DownfallProject/Core/Map/Settings/ST_LandSettings` (`.LandSettings_10_C2292C68434BF2A2A2BC62AEF734BE6D` (break `/Game/DownfallProject/Core/Map/Settings/ST_MapSettings` _settings_2)))))))
      (`KismetArrayLibrary.Array_Add` (`self.UV0`) (`KismetMathLibrary.MakeVector2D` (* (`local.X`) (`.UVScale_19_40BA05704A7CF0A676E13FB8252BB641` (break `/Game/DownfallProject/Core/Map/Settings/ST_LandSettings` (`.LandSettings_10_C2292C68434BF2A2A2BC62AEF734BE6D` (break `/Game/DownfallProject/Core/Map/Settings/ST_MapSettings` _settings_2))))) (* (`local.Y`) (`.UVScale_19_40BA05704A7CF0A676E13FB8252BB641` (break `/Game/DownfallProject/Core/Map/Settings/ST_LandSettings` (`.LandSettings_10_C2292C68434BF2A2A2BC62AEF734BE6D` (break `/Game/DownfallProject/Core/Map/Settings/ST_MapSettings` _settings_2))))))))
    (`KismetArrayLibrary.Array_Add` (`self.VerticeForNextSpace`) (`|GetArrayItem` _vertices (- (`KismetArrayLibrary.Array_Length` _vertices) 1))))
  (if (`.HasRiver_24_A6AAF5F54BFADA9B0BD3CDADA1DF578B` (break `/Game/DownfallProject/Core/Map/Settings/ST_LandSettings` (`.LandSettings_10_C2292C68434BF2A2A2BC62AEF734BE6D` (break `/Game/DownfallProject/Core/Map/Settings/ST_MapSettings` _settings))))
    (set `self.XRiver` (`KismetMathLibrary.RandomIntegerInRange` 1 (- (`self.XSize`) (+ (`self.RiverThickness`) 1))))
    (for _index_3 (range (+ (`.YSize_16_236BBE6B408435D9FF59C4AC3005C7D5` (break `/Game/DownfallProject/Core/Map/Settings/ST_LandSettings` (`.LandSettings_10_C2292C68434BF2A2A2BC62AEF734BE6D` (break `/Game/DownfallProject/Core/Map/Settings/ST_MapSettings` _settings)))) 1))
      (for _index_4 (range (`self.RiverThickness`))
        (bind _returnvalue_3 (+ (+ (* (`self.XRiver`) (+ (`.YSize_16_236BBE6B408435D9FF59C4AC3005C7D5` (break `/Game/DownfallProject/Core/Map/Settings/ST_LandSettings` (`.LandSettings_10_C2292C68434BF2A2A2BC62AEF734BE6D` (break `/Game/DownfallProject/Core/Map/Settings/ST_MapSettings` _settings)))) 1)) _index_3) (* (+ (`.YSize_16_236BBE6B408435D9FF59C4AC3005C7D5` (break `/Game/DownfallProject/Core/Map/Settings/ST_LandSettings` (`.LandSettings_10_C2292C68434BF2A2A2BC62AEF734BE6D` (break `/Game/DownfallProject/Core/Map/Settings/ST_MapSettings` _settings)))) 1) _index_4)))
        (bind (_output_x _output_y) (`KismetMathLibrary.BreakVector` (`|GetArrayItem` (`self.Vertices`) _returnvalue_3)))
        (`KismetArrayLibrary.Array_Set` (`self.Vertices`) _returnvalue_3 (`KismetMathLibrary.MakeVector` _output_x _output_y (`self.RiverHeight`))))
      (if (!= _index_3 (`.YSize_16_236BBE6B408435D9FF59C4AC3005C7D5` (break `/Game/DownfallProject/Core/Map/Settings/ST_LandSettings` (`.LandSettings_10_C2292C68434BF2A2A2BC62AEF734BE6D` (break `/Game/DownfallProject/Core/Map/Settings/ST_MapSettings` _settings)))))
        (if (and (== _returnvalue 0) (!= _returnvalue_2 (- (`self.XSize`) (+ (`self.RiverThickness`) 1))))
          (set `self.XRiver` _returnvalue_2)
          (elif (and (== _returnvalue 1) (!= (- (`self.XRiver`) 1) 0))
            (set `self.XRiver` (- (`self.XRiver`) 1))))))
    (for _index_5 (range (`self.RiverThickness`))
      (bind _returnvalue_4 (+ (`self.XRiver`) _index_5))
      (bind (_output_x_2 _output_y_2) (`KismetMathLibrary.BreakVector` (`|GetArrayItem` _verticefornextspace _returnvalue_4)))
      (`KismetArrayLibrary.Array_Set` _verticefornextspace _returnvalue_4 (`KismetMathLibrary.MakeVector` _output_x_2 _output_y_2 (`self.RiverHeight`))))))

(fn `CreateNewSpace`
  (locals (X :type Integer) (Y :type Integer) (Compt :type Integer) (Temp :type "/Game/DownfallProject/Core/Map/BP_MapSpawner Object Reference") (NewSettings :type "/Game/DownfallProject/Core/Map/Settings/ST_MapSettings Structure") (Rarity :type Integer))
  (bind _returnvalue (`KismetMathLibrary.RandomIntegerInRange` 0 2))
  (bind _temp (`local.Temp`))
  (bind _temp_2 (`local.Temp`))
  (bind _temp_3 (`local.Temp`))
  (bind _verticefornextspace (`self.VerticeForNextSpace`))
  (bind _temp_4 (`local.Temp`))
  (bind _compt (`local.Compt`))
  (bind _temp_5 (`local.Temp`))
  (bind (_returnvalue_x _returnvalue_y) (`KismetMathLibrary.BreakVector` (`SceneComponent.K2_GetComponentLocation` (`self.ProceduralMesh`))))
  (bind (_returnvalue_x_2 _returnvalue_y_2 _returnvalue_z) (`KismetMathLibrary.BreakVector` (`self.K2_GetActorLocation` _temp_3)))
  (bind (_output_x _output_y _output_z) (`KismetMathLibrary.BreakVector` (`|GetArrayItem` _verticefornextspace)))
  (bind _settings (`/Game/DownfallProject/Core/Map/Settings/MapSettings.Settings` (`self.MapSettingsActor`)))
  (bind _vertices (`/Game/DownfallProject/Core/Map/BP_MapSpawner.Vertices` _temp_2))
  (bind _settings_2 (`/Game/DownfallProject/Core/Map/BP_MapSpawner.Settings` (`local.Temp`)))
  (bind _verticefornextspace_2 (`/Game/DownfallProject/Core/Map/BP_MapSpawner.VerticeForNextSpace` (`local.Temp`)))
  (bind _settings_3 (`/Game/DownfallProject/Core/Map/BP_MapSpawner.Settings` _temp_5))
  (bind _settings_4 (`/Game/DownfallProject/Core/Map/BP_MapSpawner.Settings` (`local.Temp`)))
  (bind _returnvalue_2 (`KismetArrayLibrary.Array_Length` _settings))
  (bind _returnvalue_3 (+ (`/Game/DownfallProject/Core/Map/BP_MapSpawner.XRiver` (`local.Temp`)) 1))
  (bind _returnvalue_4 (`|SpawnActorFromClass` "BP_MapSpawner_C" (`KismetMathLibrary.MakeTransform` (`KismetMathLibrary.MakeVector` 0.0 (+ _returnvalue_y (* (`self.YSize`) (`self.ScaleY`))))) "Undefined" "OverrideRootScale" null null))
  (bind _output_get (set `local.Temp` _returnvalue_4))
  (set `/Game/DownfallProject/Core/Map/BP_MapSpawner.XSize` (`self.XSize`) _output_get)
  (set `/Game/DownfallProject/Core/Map/BP_MapSpawner.ScaleX` (`self.ScaleX`) _output_get)
  (set `/Game/DownfallProject/Core/Map/BP_MapSpawner.ScaleY` (`self.ScaleY`) _output_get)
  (set `/Game/DownfallProject/Core/Map/BP_MapSpawner.RiverHeight` (`self.RiverHeight`) _output_get)
  (set `/Game/DownfallProject/Core/Map/BP_MapSpawner.RiverThickness` (`self.RiverThickness`) _output_get)
  (set `/Game/DownfallProject/Core/Map/BP_MapSpawner.MapSettingsActor` (`self.MapSettingsActor`) _output_get)
  (for _index (range (+ _returnvalue_2 1))
    (bind (_output_enum _output_landsettings _output_spawnersettings _output_rarity) (break `/Game/DownfallProject/Core/Map/Settings/ST_MapSettings` (`|GetArrayItem` _settings _index)))
    (set `local.Rarity` (+ _output_rarity (`local.Rarity`))))
  (bind _output_get_2 (set `local.Rarity` (`KismetMathLibrary.RandomIntegerInRange` 0 (`local.Rarity`))))
  (for _index_2 (range (+ _returnvalue_2 1))
    (bind (_output_enum_2 _output_landsettings_2 _output_spawnersettings_2 _output_rarity_2) (break `/Game/DownfallProject/Core/Map/Settings/ST_MapSettings` (`|GetArrayItem` (`/Game/DownfallProject/Core/Map/Settings/MapSettings.Settings` (`self.MapSettingsActor`)) _index_2)))
    (if (<= _output_get_2 _output_rarity_2)
      (break)
      (else
        (set `local.Rarity` (- (`local.Rarity`) _output_rarity_2)))))
  (bind _output_get_3 (set `/Game/DownfallProject/Core/Map/BP_MapSpawner.Settings` (`|GetArrayItem` (`/Game/DownfallProject/Core/Map/Settings/MapSettings.Settings` (`self.MapSettingsActor`)) _index_2) _output_get))
  (if (and (`.HasRiver_24_A6AAF5F54BFADA9B0BD3CDADA1DF578B` (break `/Game/DownfallProject/Core/Map/Settings/ST_LandSettings` (`.LandSettings_10_C2292C68434BF2A2A2BC62AEF734BE6D` (break `/Game/DownfallProject/Core/Map/Settings/ST_MapSettings` _output_get_3)))) (`.HasRiver_24_A6AAF5F54BFADA9B0BD3CDADA1DF578B` (break `/Game/DownfallProject/Core/Map/Settings/ST_LandSettings` (`.LandSettings_10_C2292C68434BF2A2A2BC62AEF734BE6D` (break `/Game/DownfallProject/Core/Map/Settings/ST_MapSettings` (`self.Settings`))))))
    (set `/Game/DownfallProject/Core/Map/BP_MapSpawner.XRiver` (`self.XRiver`) (`local.Temp`)))
  (for _index_3 (range (+ (`self.XSize`) 1))
    (set `local.X` _index_3)
    (for _index_4 (range (+ (`self.YSize`) 1))
      (set `local.Y` _index_4)
      (if (or (== _compt 0) (== (mod _compt (+ (`self.YSize`) 1)) 0))
        (`KismetArrayLibrary.Array_Add` (`/Game/DownfallProject/Core/Map/BP_MapSpawner.Vertices` (`local.Temp`)) (`KismetMathLibrary.MakeVector` (* (`local.X`) (`self.ScaleX`)) (* (`local.Y`) (`self.ScaleY`)) _output_z))
        (`KismetArrayLibrary.Array_Remove` _verticefornextspace)
        (`/Engine/EditorBlueprintResources/StandardMacros.IncrementInt` (`local.Compt`))
        (else
          (`KismetArrayLibrary.Array_Add` (`/Game/DownfallProject/Core/Map/BP_MapSpawner.Vertices` _temp_4) (`KismetMathLibrary.MakeVector` (* (`local.X`) (`self.ScaleX`)) (* (`local.Y`) (`self.ScaleY`)) (`KismetMathLibrary.RandomFloatInRange` (`.ZMin_20_EBE479EB4E5073A8409F7B9CB26DAF67` (break `/Game/DownfallProject/Core/Map/Settings/ST_LandSettings` (`.LandSettings_10_C2292C68434BF2A2A2BC62AEF734BE6D` (break `/Game/DownfallProject/Core/Map/Settings/ST_MapSettings` _settings_4)))) (`.ZMax_21_6862E78A47B566DFAEF57B9A59C42546` (break `/Game/DownfallProject/Core/Map/Settings/ST_LandSettings` (`.LandSettings_10_C2292C68434BF2A2A2BC62AEF734BE6D` (break `/Game/DownfallProject/Core/Map/Settings/ST_MapSettings` _settings_4)))))))
          (`KismetArrayLibrary.Array_Add` (`/Game/DownfallProject/Core/Map/BP_MapSpawner.UV0` _temp_4) (`KismetMathLibrary.MakeVector2D` (* (`local.X`) (`.UVScale_19_40BA05704A7CF0A676E13FB8252BB641` (break `/Game/DownfallProject/Core/Map/Settings/ST_LandSettings` (`.LandSettings_10_C2292C68434BF2A2A2BC62AEF734BE6D` (break `/Game/DownfallProject/Core/Map/Settings/ST_MapSettings` _settings_4))))) (* (`local.Y`) (`.UVScale_19_40BA05704A7CF0A676E13FB8252BB641` (break `/Game/DownfallProject/Core/Map/Settings/ST_LandSettings` (`.LandSettings_10_C2292C68434BF2A2A2BC62AEF734BE6D` (break `/Game/DownfallProject/Core/Map/Settings/ST_MapSettings` _settings_4)))))))
          (`/Engine/EditorBlueprintResources/StandardMacros.IncrementInt` (`local.Compt`)))))
    (`KismetArrayLibrary.Array_Add` (`/Game/DownfallProject/Core/Map/BP_MapSpawner.VerticeForNextSpace` _temp_2) (`|GetArrayItem` _vertices (- (`KismetArrayLibrary.Array_Length` _vertices) 1))))
  (if (`.HasRiver_24_A6AAF5F54BFADA9B0BD3CDADA1DF578B` (break `/Game/DownfallProject/Core/Map/Settings/ST_LandSettings` (`.LandSettings_10_C2292C68434BF2A2A2BC62AEF734BE6D` (break `/Game/DownfallProject/Core/Map/Settings/ST_MapSettings` _settings_3))))
    (if (not (!= (`/Game/DownfallProject/Core/Map/BP_MapSpawner.XRiver` _temp_5) 0))
      (set `/Game/DownfallProject/Core/Map/BP_MapSpawner.XRiver` (`KismetMathLibrary.RandomIntegerInRange` 1 (- (`self.XSize`) (`self.RiverThickness`))) (`local.Temp`)))
    (for _index_5 (range (+ (`.YSize_16_236BBE6B408435D9FF59C4AC3005C7D5` (break `/Game/DownfallProject/Core/Map/Settings/ST_LandSettings` (`.LandSettings_10_C2292C68434BF2A2A2BC62AEF734BE6D` (break `/Game/DownfallProject/Core/Map/Settings/ST_MapSettings` _settings_3)))) 1))
      (for _index_6 (range (`self.RiverThickness`))
        (bind _returnvalue_5 (+ (+ (* (`/Game/DownfallProject/Core/Map/BP_MapSpawner.XRiver` (`local.Temp`)) (+ (`.YSize_16_236BBE6B408435D9FF59C4AC3005C7D5` (break `/Game/DownfallProject/Core/Map/Settings/ST_LandSettings` (`.LandSettings_10_C2292C68434BF2A2A2BC62AEF734BE6D` (break `/Game/DownfallProject/Core/Map/Settings/ST_MapSettings` _settings_3)))) 1)) _index_5) (* (+ (`.YSize_16_236BBE6B408435D9FF59C4AC3005C7D5` (break `/Game/DownfallProject/Core/Map/Settings/ST_LandSettings` (`.LandSettings_10_C2292C68434BF2A2A2BC62AEF734BE6D` (break `/Game/DownfallProject/Core/Map/Settings/ST_MapSettings` _settings_3)))) 1) _index_6)))
        (bind (_output_x_2 _output_y_2) (`KismetMathLibrary.BreakVector` (`|GetArrayItem` (`/Game/DownfallProject/Core/Map/BP_MapSpawner.Vertices` (`local.Temp`)) _returnvalue_5)))
        (`KismetArrayLibrary.Array_Set` (`/Game/DownfallProject/Core/Map/BP_MapSpawner.Vertices` (`local.Temp`)) _returnvalue_5 (`KismetMathLibrary.MakeVector` _output_x_2 _output_y_2 (`self.RiverHeight`))))
      (if (!= _index_5 (`.YSize_16_236BBE6B408435D9FF59C4AC3005C7D5` (break `/Game/DownfallProject/Core/Map/Settings/ST_LandSettings` (`.LandSettings_10_C2292C68434BF2A2A2BC62AEF734BE6D` (break `/Game/DownfallProject/Core/Map/Settings/ST_MapSettings` _settings_3)))))
        (if (and (== _returnvalue 0) (!= _returnvalue_3 (- (`self.XSize`) (+ (`self.RiverThickness`) 1))))
          (set `/Game/DownfallProject/Core/Map/BP_MapSpawner.XRiver` _returnvalue_3 (`local.Temp`))
          (elif (and (== _returnvalue 1) (!= (- (`/Game/DownfallProject/Core/Map/BP_MapSpawner.XRiver` (`local.Temp`)) 1) 0))
            (set `/Game/DownfallProject/Core/Map/BP_MapSpawner.XRiver` (- (`/Game/DownfallProject/Core/Map/BP_MapSpawner.XRiver` (`local.Temp`)) 1) (`local.Temp`))))))
    (for _index_7 (range (`self.RiverThickness`))
      (bind _returnvalue_6 (+ (`/Game/DownfallProject/Core/Map/BP_MapSpawner.XRiver` (`local.Temp`)) _index_7))
      (bind (_output_x_3 _output_y_3) (`KismetMathLibrary.BreakVector` (`|GetArrayItem` _verticefornextspace_2 _returnvalue_6)))
      (`KismetArrayLibrary.Array_Set` _verticefornextspace_2 _returnvalue_6 (`KismetMathLibrary.MakeVector` _output_x_3 _output_y_3 (`self.RiverHeight`)))))
  (`self.CreateTriangles` _temp_3)
  (`ProceduralMeshComponent.CreateMeshSection_LinearColor` :`self` (`/Game/DownfallProject/Core/Map/BP_MapSpawner.ProceduralMesh` _temp_3) :`Vertices` (`/Game/DownfallProject/Core/Map/BP_MapSpawner.Vertices` _temp_3) :`Triangles` (`/Game/DownfallProject/Core/Map/BP_MapSpawner.Triangles` _temp_3) :`UV0` (`/Game/DownfallProject/Core/Map/BP_MapSpawner.UV0` _temp_3) :`bCreateCollision` true)
  (bind _returnvalue_7 (`|SpawnActorFromClass` "/Game/DownfallProject/Core/Map/BP_SpawnObjectOnMap.BP_SpawnObjectOnMap_C" (`KismetMathLibrary.MakeTransform` (`KismetMathLibrary.MakeVector` (+ (/ (* (`self.XSize`) (`self.ScaleX`)) 2.0) _returnvalue_x_2) (+ _returnvalue_y_2 (/ (* (`self.YSize`) (`self.ScaleY`)) 2.0)) (+ _returnvalue_z (`self.ZMax`))) (struct) (`KismetMathLibrary.MakeVector` (/ (* (`self.XSize`) (`self.ScaleX`)) 1000.0) (/ (* (`self.YSize`) (`self.ScaleY`)) 1000.0) 1.0)) "Undefined" "OverrideRootScale" null null))
  (`self.K2_AttachToActor` _returnvalue_7 (`local.Temp`) "None" "KeepWorld" "KeepWorld" "KeepWorld" true)
  (if (== (`self.NbMap`) (`self.NbMapToUpDifficulty`))
    (set `self.NbMap` 0)
    (bind _output_get_4 (set `/Game/DownfallProject/Core/Map/BP_MapSpawner.CurrentMultiplierDifficulty` (* (`self.CurrentMultiplierDifficulty`) (`self.MultiplierDifficulty`)) _temp))
    (else
      (set `/Game/DownfallProject/Core/Map/BP_MapSpawner.CurrentMultiplierDifficulty` (`self.CurrentMultiplierDifficulty`) _temp)))
  (for (_array_element _array_index) (`.Nb_6_C1DBD6824FD7A42454408BB1173DBCFA` (break `/Game/DownfallProject/Core/Map/Settings/ST_SpawnerSettings` (`.SpawnerSettings_7_E9E668DB4E30D507BFFFB4ACE8597935` (break `/Game/DownfallProject/Core/Map/Settings/ST_MapSettings` (`/Game/DownfallProject/Core/Map/BP_MapSpawner.Settings` (`local.Temp`))))))
    (`KismetArrayLibrary.Array_Set` (`.Nb_6_C1DBD6824FD7A42454408BB1173DBCFA` (break `/Game/DownfallProject/Core/Map/Settings/ST_SpawnerSettings` (`.SpawnerSettings_7_E9E668DB4E30D507BFFFB4ACE8597935` (break `/Game/DownfallProject/Core/Map/Settings/ST_MapSettings` _settings_2)))) _array_index (* _array_element _output_get_4)))
  (set `/Game/DownfallProject/Core/Map/BP_SpawnObjectOnMap.Settings` (make `/Game/DownfallProject/Core/Map/Settings/ST_SpawnerSettings` (break `/Game/DownfallProject/Core/Map/Settings/ST_SpawnerSettings` (`.SpawnerSettings_7_E9E668DB4E30D507BFFFB4ACE8597935` (break `/Game/DownfallProject/Core/Map/Settings/ST_MapSettings` _settings_2))) (`.Nb_6_C1DBD6824FD7A42454408BB1173DBCFA` (break `/Game/DownfallProject/Core/Map/Settings/ST_SpawnerSettings` (`.SpawnerSettings_7_E9E668DB4E30D507BFFFB4ACE8597935` (break `/Game/DownfallProject/Core/Map/Settings/ST_MapSettings` _settings_2))))) _returnvalue_7)
  (set `/Game/DownfallProject/Core/Map/BP_MapSpawner.NbMap` (+ (`self.NbMap`) 1) _temp)
  (`/Game/DownfallProject/Core/Map/BP_SpawnObjectOnMap.Spawn` _returnvalue_7)
  (`PrimitiveComponent.SetMaterial` (`/Game/DownfallProject/Core/Map/BP_MapSpawner.ProceduralMesh` (`local.Temp`)) 0 (break `/Game/DownfallProject/Core/Map/Settings/ST_LandSettings` (`.LandSettings_10_C2292C68434BF2A2A2BC62AEF734BE6D` (break `/Game/DownfallProject/Core/Map/Settings/ST_MapSettings` (`/Game/DownfallProject/Core/Map/BP_MapSpawner.Settings` (`local.Temp`))))))
  (set `self.ObjectSpawner` _returnvalue_7)
  (set `/Game/DownfallProject/Core/Map/BP_MapSpawner.EndConstruct` true (`local.Temp`)))

(fn `CreateTriangles`
  (locals (Vertex :type Integer))
  (for _ (range (`self.XSize`))
    (for _ (range (`self.YSize`))
      (`KismetArrayLibrary.Array_Add` (`self.Triangles`) (`local.Vertex`))
      (`KismetArrayLibrary.Array_Add` (`self.Triangles`) (+ (`local.Vertex`) 1))
      (`KismetArrayLibrary.Array_Add` (`self.Triangles`) (+ (`self.YSize`) 1 (`local.Vertex`)))
      (`KismetArrayLibrary.Array_Add` (`self.Triangles`) (+ (`local.Vertex`) 1))
      (`KismetArrayLibrary.Array_Add` (`self.Triangles`) (+ (`self.YSize`) 2 (`local.Vertex`)))
      (`KismetArrayLibrary.Array_Add` (`self.Triangles`) (+ (`self.YSize`) 1 (`local.Vertex`)))
      (`/Engine/EditorBlueprintResources/StandardMacros.IncrementInt` (`local.Vertex`)))
    (`/Engine/EditorBlueprintResources/StandardMacros.IncrementInt` (`local.Vertex`))))

(fn `UserConstructionScript`)